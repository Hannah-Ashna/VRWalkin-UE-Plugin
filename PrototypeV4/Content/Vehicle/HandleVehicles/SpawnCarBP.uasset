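; SpawnCarBP is a vehicle spawner that keeps the level populated with BP_Hatchback cars.
; Tick counts all hatchbacks and, while there are fewer than four, spawns one at the SpawnerVolume transform and gives it a default controller.
; BeginPlay also sets a looping timer for SpawnCarActor on SpawnerVolume, a function this Blueprint does not define, so spawning here runs from Tick.
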(event EventBeginPlay
  (Utilities|Time|SetTimerbyFunctionName (Variables|Default|GetSpawner%20Volume) "SpawnCarActor" 2e+01 true))

(event EventTick
  (params (DeltaSeconds :type Float%20%28single-precision%29))
  (bind _outactors (Actor|GetAllActorsOfClass "/Game/VehicleVarietyPack/Blueprints/Hatchback/BP_Hatchback.BP_Hatchback_C"))
  (if (< (Utilities|Array|Length _outactors) 4)
    (bind _returnvalue (Game|SpawnActorfromClass "/Game/VehicleVarietyPack/Blueprints/Hatchback/BP_Hatchback.BP_Hatchback_C" (Transformation|GetWorldTransform (Variables|Default|GetSpawner%20Volume)) "Undefined" 0 0))
    (Utilities|IsValid _returnvalue
      (:Is%20Valid
        (Pawn|SpawnDefaultController _returnvalue)))))

(fn ConstructionScript)