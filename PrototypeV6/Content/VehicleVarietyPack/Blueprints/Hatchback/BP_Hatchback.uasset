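; BP_Hatchback is an AI-driven traffic car that follows the ActivePath spline and stops for obstacles and other hatchbacks.
; Each tick, GetPath looks 500 units ahead along the spline tangent and maps the yaw error to steering input.
; Driving applies Speed as throttle, while Stop cuts throttle and sets the handbrake.
; FrontSensor overlaps toggle these, and seeing another BP_Hatchback stops it, resuming after a retriggerable 1.5-second delay.
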(event OnSeePawn(PawnSensing)
  (params (Pawn :type Pawn%20Object%20Reference))
  ;[1 1 1] Stop Car
  (Utilities|Casting|CastToBP_Hatchback Pawn)
  (Utilities|FlowControl|Sequence
    (:then_0
      (CallFunction|Stop))
    (:then_1
      (Utilities|FlowControl|RetriggerableDelay 1.5)
      (CallFunction|Driving))))

(event OnComponentBeginOverlap(FrontSensor)
  (params (OverlappedComponent :type Primitive%20Component%20Object%20Reference) (OtherActor :type Actor%20Object%20Reference) (OtherComp :type Primitive%20Component%20Object%20Reference) (OtherBodyIndex :type Integer) (bFromSweep :type Boolean) (SweepResult :type Hit%20Result%20Structure%20%28by%20ref%29))
  ;[1 1 1] Sensors
  (CallFunction|Stop))

(event OnComponentEndOverlap(FrontSensor)
  (params (OverlappedComponent :type Primitive%20Component%20Object%20Reference) (OtherActor :type Actor%20Object%20Reference) (OtherComp :type Primitive%20Component%20Object%20Reference) (OtherBodyIndex :type Integer))
  ;[1 1 1] Sensors
  (CallFunction|Driving))

(event EventBeginPlay
  ;[1 1 1] Spawn Car
  (CallFunction|Driving))

(event EventTick
  (params (DeltaSeconds :type Float%20%28single-precision%29))
  ;[1 1 1] Steering input
  (bind _steering (CallFunction|GetPath))
  (Class|WheeledVehicleMovementComponent|SetSteeringInput (Variables|Default|GetVehicleMovement) _steering))

(fn ConstructionScript)

(fn Stop
  (bind _vehiclemovement (Variables|Default|GetVehicleMovement))
  (Class|WheeledVehicleMovementComponent|SetThrottleInput _vehiclemovement 0.0)
  (bind _output_get (Variables|Default|SetStand true))
  (Class|WheeledVehicleMovementComponent|SetHandbrakeInput _vehiclemovement _output_get))

(fn Driving
  (bind _vehiclemovement (Variables|Default|GetVehicleMovement))
  (bind _output_get (Variables|Default|SetStand false))
  (Class|WheeledVehicleMovementComponent|SetHandbrakeInput _vehiclemovement _output_get)
  (Class|WheeledVehicleMovementComponent|SetThrottleInput _vehiclemovement (Variables|Default|GetSpeed)))

(fn GetPath
  (bind _returnvalue (Transformation|GetActorLocation))
  (bind _active_path (Variables|Components|GetActive%20Path))
  (Utilities|IsValid _active_path
    (:Is%20Valid
      (return (Math|Float|MapRangeClamped (.yaw (Math|Rotator|Delta(Rotator) (Math|Rotator|FindLookatRotation _returnvalue (Spline|FindLocationClosesttoWorldLocation _active_path (+ (* (Math|Vector|Normalize (Class|SplineComponent|FindTangentClosesttoWorldLocation _active_path _returnvalue "World")) 5e+02) _returnvalue) "World")) (Transformation|GetActorRotation))) -9e+01 9e+01 -1.0 1.0)))))